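; BP_WheelPawn is a possessable interaction pawn that lets the player turn a BP_WheelToOpen with the mouse cursor.
; While the mouse input is held, it picks the wheel under the cursor, then rolls it to the cursor's angle around the wheel's projected screen center until it peaks.
; A spinning sound plays during turning and pauses otherwise.
; Interact or ForceExit calls the wheel's WallGoDown and repossesses the first-person character.
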(event `self.ReceiveBeginPlay`
  ; Looks For Player
  (bind _asbp_first_person_character (cast `/Game/FirstPerson/Blueprints/BP_FirstPersonCharacter` (`GameplayStatics.GetPlayerPawn` 0)))
  (set `self.DefaultPlayer` _asbp_first_person_character)
  (bind _returnvalue (`AddComponent|NODE_AddAudioComponent-1`))
  (bind _output_get (set `self.SpiningWheel` _returnvalue))
  (`AudioComponent.Stop` _output_get))

(event `self.ReceivePossessed`
  (params (NewController :type "Controller Object Reference"))
  ; Reset inputs when being possessed
  (bind _asbp_first_person_player_controller (cast `/Game/FirstPerson/Blueprints/BP_FirstPersonPlayerController` NewController))
  (`/Game/FirstPerson/Blueprints/BP_FirstPersonPlayerController.Reset_Input` _asbp_first_person_player_controller false)
  (set `PlayerController.bShowMouseCursor` true _asbp_first_person_player_controller)
  (set `/Game/FirstPerson/Blueprints/BP_FirstPersonCharacter.WheelPawn` self (`self.DefaultPlayer`)))

(event `EnhancedInput|/Game/Input/Actions/IA_Interact`
  (params (ActionValue :type Boolean) (ElapsedSeconds :type "Float (double-precision)") (TriggeredSeconds :type "Float (double-precision)") (InputAction :type "InputAction Object Reference" :default "/Game/Input/Actions/IA_Interact.IA_Interact"))
  (bind _defaultplayer (`self.DefaultPlayer`))
  ; Exits Pawn to go  back to regular player
  (:`Triggered`
    (if (not (`self.Transitioning`)) :!label _label
      (bind _wheelactor (`self.WheelActor`)
        (:`then`
          (`/Game/Blueprint/Functionality/BP_WheelToOpen.WallGoDown` _wheelactor)
          (`AudioComponent.Stop` (`self.SpiningWheel`)))
        (:`else`
          _))
      (set `/Game/FirstPerson/Blueprints/BP_FirstPersonCharacter.isInteracting ` true _defaultplayer)
      (`Controller.Possess` (`GameplayStatics.GetPlayerController` 0) _defaultplayer)
      (`KismetSystemLibrary.Delay` 0.2)
      (set `/Game/FirstPerson/Blueprints/BP_FirstPersonCharacter.isInteracting ` false (`self.DefaultPlayer`))
      (`self.ResetVariables`))))

(event `ForceExit`
  ; Exits Pawn to go  back to regular player
  (`KismetSystemLibrary.PrintString` "Forfce ex" true true (struct :`G` 0.66 :`B` 1.0 :`A` 1.0) 1000.0)
  (set `/Game/FirstPerson/Blueprints/BP_FirstPersonCharacter.WheelPawn` null (`self.DefaultPlayer`))
  (goto _label))

(event `ResetVariables`
  (set `self.landedOnWheel` false)
  (set `self.WheelActor` null))

(event `PauseAudio`
  (`AudioComponent.SetPaused` (`self.SpiningWheel`) true))

(event `EnhancedInput|/Game/Input/Actions/IA_MouseWheel`
  (params (ActionValue :type Boolean) (ElapsedSeconds :type "Float (double-precision)") (TriggeredSeconds :type "Float (double-precision)") (InputAction :type "InputAction Object Reference" :default "/Game/Input/Actions/IA_MouseWheel.IA_MouseWheel"))
  (bind _returnvalue (`GameplayStatics.GetPlayerController` 0))
  (bind (_locationx _locationy) (`PlayerController.GetMousePosition` _returnvalue))
  ; BS
  (:`Triggered`
    (bind _wheelactor (`self.WheelActor`)
      (:`then`
        (if (not (`/Game/Blueprint/Functionality/BP_WheelToOpen.Peak` _wheelactor))
          (if (not (`self.landedOnWheel`)) :!label _label_2
            (bind _asbp_wheel_to_open (cast `/Game/Blueprint/Functionality/BP_WheelToOpen` (`.HitActor` (`GameplayStatics.BreakHitResult` (`PlayerController.GetHitResultUnderCursorByChannel` _returnvalue "TraceTypeQuery1" true)))))
            (set `self.WheelActor` _asbp_wheel_to_open)
            (set `self.landedOnWheel` true)
            (`AudioComponent.Play` (`self.SpiningWheel`) 0.0)
            (else
              (bind _wheelactor_2 (`self.WheelActor`)
                (:`then`
                  (`self.ContinueAudio`)
                  (bind _wheel (`/Game/Blueprint/Functionality/BP_WheelToOpen.Wheel` _wheelactor_2))
                  (bind (_x _y) (`KismetMathLibrary.BreakVector2D` (`GameplayStatics.ProjectWorldToScreen` _returnvalue (`SceneComponent.K2_GetComponentLocation` _wheel) true)))
                  (bind (_returnvalue_roll _returnvalue_pitch _returnvalue_yaw) (`KismetMathLibrary.BreakRotator` (`SceneComponent.K2_GetComponentRotation` _wheel)))
                  (`SceneComponent.K2_SetWorldRotation` _wheel (`KismetMathLibrary.MakeRotator` (`KismetMathLibrary.DegAtan2` (- _locationx _x) (- _locationy _y)) _returnvalue_pitch _returnvalue_yaw) false false))
                (:`else`))))
          (else
            (`self.PauseAudio` :!label _label_3))))
      (:`else`
        (goto _label_2))))
  (:`Canceled`
    (goto _label_3))
  (:`Completed`
    (goto _label_3)))

(event `ContinueAudio`
  (`AudioComponent.SetPaused` (`self.SpiningWheel`) false))

(fn `UserConstructionScript`)