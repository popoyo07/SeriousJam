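; BP_CheckToShake is a trigger actor that shakes the first-person player's camera when a BP_Boulder enters its box.
; On BeginPlay it caches the player controller and character and binds to the character's Respawn event.
; A Shaking flag makes the shake fire once, with a debug "Hello" print, until a respawn resets the flag and rearms the trigger.
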(event `self.ReceiveBeginPlay`
  (bind _asbp_first_person_player_controller (cast `/Game/FirstPerson/Blueprints/BP_FirstPersonPlayerController` (`GameplayStatics.GetPlayerController` 0)))
  (set `self.PlayerController` _asbp_first_person_player_controller)
  (bind _asbp_first_person_character (cast `/Game/FirstPerson/Blueprints/BP_FirstPersonCharacter` (`GameplayStatics.GetPlayerPawn` 0)))
  (bind _output_get (set `self.PlayerPawn` _asbp_first_person_character))
  (add `/Game/FirstPerson/Blueprints/BP_FirstPersonCharacter.Respawn` _output_get (delegate `ResetThingy`)))

(event `ResetThingy`
  (params (SaveGame :type "/Game/Blueprint/Save/BP_Save Object Reference"))
  (set `self.Shaking` false))

(event `self.Box.OnComponentBeginOverlap`
  (params (OverlappedComponent :type "PrimitiveComponent Object Reference") (OtherActor :type "Actor Object Reference") (OtherComp :type "PrimitiveComponent Object Reference") (OtherBodyIndex :type Integer) (bFromSweep :type Boolean) (SweepResult :type "HitResult Structure (by ref)"))
  (bind _returnvalue (`GameplayStatics.ObjectIsA` OtherActor "/Game/Blueprint/Functionality/Boulder/BP_Boulder.BP_Boulder_C"))
  (if (`self.Shaking`)
    _
    (elif _returnvalue
      (set `self.Shaking` true)
      (`PlayerController.ClientStartCameraShake` :`self` (`self.PlayerController`) :`Shake` "/Game/Blueprint/Functionality/BP_CameraShaker.BP_CameraShaker_C" :`PlaySpace` "World")
      (`KismetSystemLibrary.PrintString` "Hello" _returnvalue))))

(fn `UserConstructionScript`)