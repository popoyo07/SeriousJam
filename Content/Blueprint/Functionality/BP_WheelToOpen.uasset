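; Wheel interactable that hands control to an assigned pawn and raises a linked wall in steps.
; Each box overlap by the invisible mesh increments a counter, and a timeline lifts the wall to that step's offset height.
; WallGoDown lowers it with falling audio; reaching the max count locks further raises and plays peak audio.
; Player respawn snaps the wall back and resets wheel and pawn state.
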(event `WallGoDown`
  (`AudioComponent.SetPaused` (`self.PeakSfx`) true)
  (bind _wall (`self.Wall`)
    (:`then`
      (`AudioComponent.SetPaused` (`self.FallingWallSFX`) false)
      (set `self.CurrentCount` 0)
      (set `self.WallCurrentLocation` (`self.K2_GetActorLocation` _wall))
      (`KismetSystemLibrary.PrintString` "GOing doqwn " true true (struct :`G` 0.66 :`B` 1.0 :`A` 1.0) 1000.0)
      (bind (_direction _lerptime_) (`Timeline|GoDownTimeLine` :!via `PlayFromStart` :!label _label)
        (:`Update`
          (`self.K2_SetActorLocation` (`self.Wall`) (`KismetMathLibrary.VLerp` (`self.WallCurrentLocation`) (`self.WallStartingLocation`) _lerptime_) false false))
        (:`Finished`
          (`KismetSystemLibrary.PrintString` "Went down ")
          (set `self.CurrentCount` 0)
          (set `self.CoolDown` false)
          (set `self.Peak` false))))
    (:`else`)))

(event `ForceStop`
  (goto _label :!via `Stop`))

(event `/Game/Blueprint/Functionality/BPI_Interact.Interact`
  (params (Player :type "/Game/FirstPerson/Blueprints/BP_FirstPersonCharacter Object Reference"))
  (bind _player (`self.Player`))
  ; Interact
  (bind _pawn (`self.Pawn`)
    (:`then`
      (set `/Game/Blueprint/Characters/BP_WheelPawn.Transitioning` true _pawn)
      (`Controller.Possess` (`GameplayStatics.GetPlayerController` 0) _pawn)
      (bind _billboard (`/Game/Blueprint/Characters/BP_WheelPawn.Billboard` _pawn))
      (`SceneComponent.K2_SetWorldLocation` (`Actor.RootComponent` _player) (`SceneComponent.K2_GetComponentLocation` _billboard) false true)
      (`SceneComponent.K2_SetWorldRotation` (`Actor.RootComponent` _player) (`SceneComponent.K2_GetComponentRotation` _billboard) false true)
      (`KismetSystemLibrary.Delay` 0.5)
      (set `/Game/Blueprint/Characters/BP_WheelPawn.Transitioning` false (`self.Pawn`)))
    (:`else`
      (`KismetSystemLibrary.PrintString` "You need to set pawn vraiable on editor "))))

(event `self.ReceiveBeginPlay`
  (bind _asbp_first_person_character (cast `/Game/FirstPerson/Blueprints/BP_FirstPersonCharacter` (`GameplayStatics.GetPlayerPawn` 0)))
  (set `self.Player` _asbp_first_person_character)
  (bind _wall (`self.Wall`)
    (:`then`
      (set `self.WallStartingLocation` (`self.K2_GetActorLocation` _wall))
      (set `self.LocationToGoUp` (`SceneComponent.K2_GetComponentLocation` (`self.Wall1Turn`)))
      (bind _returnvalue (`AddComponent|NODE_AddAudioComponent-1`))
      (bind _output_get (set `self.FallingWallSFX` _returnvalue))
      (`AudioComponent.SetPaused` _output_get true)
      (add `/Game/FirstPerson/Blueprints/BP_FirstPersonCharacter.Respawn` (`self.Player`) (delegate `ResetWakk`))
      (bind _returnvalue_2 (`AddComponent|NODE_AddAudioComponent-2`))
      (bind _output_get_2 (set `self.PeakSfx` _returnvalue_2))
      (`AudioComponent.SetPaused` _output_get_2 true))
    (:`else`
      (`KismetSystemLibrary.PrintString` "Set Up Wall"))))

(event `WallGoUp`
  (bind (_wallcurrentlocation_x _wallcurrentlocation_y) (`KismetMathLibrary.BreakVector` (`self.WallCurrentLocation`)))
  (bind _wall (`self.Wall`)
    (:`then`
      (set `self.WallCurrentLocation` (`self.K2_GetActorLocation` _wall))
      (bind _newparam (`self.DetermineUpLocation`))
      (`|ExecutionSequence`
        (:`then_0`
          (bind (_direction _lerp) (`Timeline|GoUp` :!via `Stop` :!label _label_2)
            (:`Update`
              (bind (_returnvalue_x _returnvalue_y _returnvalue_z) (`KismetMathLibrary.BreakVector` (`KismetMathLibrary.VLerp` (`self.WallCurrentLocation`) _newparam _lerp)))
              (`self.K2_SetActorLocation` (`self.Wall`) (`KismetMathLibrary.MakeVector` _wallcurrentlocation_x _wallcurrentlocation_y _returnvalue_z) false false))))
        (:`then_1`
          (`KismetSystemLibrary.Delay` 0.2)
          (goto _label_2 :!via `PlayFromStart`))))
    (:`else`)))

(event `ResetWakk`
  (params (SaveGame :type "/Game/Blueprint/Save/BP_Save Object Reference"))
  (`self.ForceStop`)
  (`self.K2_SetActorLocation` (`self.Wall`) (`self.WallStartingLocation`) false false)
  (`self.Reset Variables`
    (:`yee`
      (`/Game/Blueprint/Characters/BP_WheelPawn.ResetVariables` (`self.Pawn`)))))

(event `self.Box.OnComponentBeginOverlap`
  (params (OverlappedComponent :type "PrimitiveComponent Object Reference") (OtherActor :type "Actor Object Reference") (OtherComp :type "PrimitiveComponent Object Reference") (OtherBodyIndex :type Integer) (bFromSweep :type Boolean) (SweepResult :type "HitResult Structure (by ref)"))
  (if (== OtherComp (`self.InvisibleMesh`))
    (if (not (`self.Peak`))
      (if (not (`self.CoolDown`))
        (set `self.CoolDown` true)
        (bind _result (`/Engine/EditorBlueprintResources/StandardMacros.IncrementInt` (`self.CurrentCount`))
          (:`  `
            (bind _output_get (set `self.CurrentCount` _result))
            (`self.ForceStop`)
            (`self.WallGoUp`)
            (`AudioComponent.SetPaused` (`self.FallingWallSFX`) true)
            (if (== _output_get (`self.MaxCount`))
              (set `self.Peak` true)
              (`AudioComponent.SetPaused` (`self.PeakSfx`) false)
              (else
                (`KismetSystemLibrary.Delay` 0.2)
                (set `self.CoolDown` false)
                (set `self.Peak` false)))))))))

(fn `DetermineUpLocation`
  (returns (NewParam :type "Vector Structure"))
  (locals (OffSet :type "Float (double-precision)"))
  (bind (_locationtogoup_x _locationtogoup_y _locationtogoup_z) (`KismetMathLibrary.BreakVector` (`self.LocationToGoUp`)))
  (bind _currentcount (`self.CurrentCount`))
  (if (> _currentcount 0)
    (set `local.OffSet` (`|GetArrayItem` (`self.Offsets`) (- _currentcount 1)))
    (return (`KismetMathLibrary.MakeVector` _locationtogoup_x _locationtogoup_y (- _locationtogoup_z (`local.OffSet`))))))

(fn `UserConstructionScript`)