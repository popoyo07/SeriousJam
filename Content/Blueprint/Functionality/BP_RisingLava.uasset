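; Rising lava hazard that damages the first-person character when it overlaps the lava plane.
; The player entering the trigger box starts, once and after a delay, a timeline that moves the plane through LerpToBillBoard.
; The character's respawn event stops the rise, restores the plane's start location and re-arms the trigger.
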(event `StartRise`
  (bind (_direction _alpha) (`Timeline|Timeline` :!via `PlayFromStart` :!label _label)
    (:`Update`
      (`SceneComponent.K2_SetRelativeLocation` (`self.Plane`) (`self.LerpToBillBoard` _alpha) false false))))

(event `StopRise`
  (goto _label :!via `Stop`))

(event `self.ReceiveBeginPlay`
  (bind _asbp_first_person_character (cast `/Game/FirstPerson/Blueprints/BP_FirstPersonCharacter` (`GameplayStatics.GetPlayerCharacter` 0)))
  (add `/Game/FirstPerson/Blueprints/BP_FirstPersonCharacter.Respawn` _asbp_first_person_character (delegate `Reset`))
  (set `self.StartLocation` (`SceneComponent.RelativeLocation` (`self.Plane`))))

(event `Reset`
  (params (SaveGame :type "/Game/Blueprint/Save/BP_Save Object Reference"))
  (`self.StopRise`)
  (`SceneComponent.K2_SetRelativeLocation` (`self.Plane`) (`self.StartLocation`) false false)
  (`self.ResetTrigger`))

(event `self.Plane.OnComponentBeginOverlap`
  (params (OverlappedComponent :type "PrimitiveComponent Object Reference") (OtherActor :type "Actor Object Reference") (OtherComp :type "PrimitiveComponent Object Reference") (OtherBodyIndex :type Integer) (bFromSweep :type Boolean) (SweepResult :type "HitResult Structure (by ref)"))
  (bind _asbp_first_person_character (cast `/Game/FirstPerson/Blueprints/BP_FirstPersonCharacter` OtherActor))
  (`/Game/FirstPerson/Blueprints/BP_FirstPersonCharacter.TakeDamage` _asbp_first_person_character "You are swimming in lava"))

(event `self.Box.OnComponentBeginOverlap`
  (params (OverlappedComponent :type "PrimitiveComponent Object Reference") (OtherActor :type "Actor Object Reference") (OtherComp :type "PrimitiveComponent Object Reference") (OtherBodyIndex :type Integer) (bFromSweep :type Boolean) (SweepResult :type "HitResult Structure (by ref)"))
  (if (`GameplayStatics.ObjectIsA` OtherActor "/Game/FirstPerson/Blueprints/BP_FirstPersonCharacter.BP_FirstPersonCharacter_C")
    (`/Engine/EditorBlueprintResources/StandardMacros.DoOnce` false :!label _label_2
      (:`Completed`
        (`KismetSystemLibrary.Delay` (`self.LavaRiseDelay`))
        (`self.StartRise`)))))

(event `ResetTrigger`
  (goto _label_2 :!via `Reset`))

(fn `UserConstructionScript`)