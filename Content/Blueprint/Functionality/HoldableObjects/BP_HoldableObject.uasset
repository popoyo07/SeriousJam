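; BP_HoldableObject is an actor that the player can pick up, throw or place at a socket.
; Interact disables mesh physics, detaches the actor and passes it to the player's PickUpObject, only when the player holds nothing.
; ThrownObject detaches it, re-enables physics and applies the given velocity as a mass-dependent impulse.
; PlaceObject detaches it and moves it to the supplied socket transform, leaving physics untouched.
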(event `/Game/Blueprint/Functionality/BPI_Interact.Interact`
  (params (Player :type "/Game/FirstPerson/Blueprints/BP_FirstPersonCharacter Object Reference"))
  (`/Game/FirstPerson/Blueprints/BP_FirstPersonCharacter.HeldObject` Player
    (:`then`)
    (:`else`
      (`PrimitiveComponent.SetSimulatePhysics` (`self.StaticMesh`) false)
      (`self.K2_DetachFromActor` "KeepWorld" "KeepWorld" "KeepWorld")
      (`/Game/FirstPerson/Blueprints/BP_FirstPersonCharacter.PickUpObject` Player self))))

(event `ThrownObject`
  (params (Velocity :type "Vector Structure"))
  (bind _staticmesh (`self.StaticMesh`))
  (`self.K2_DetachFromActor` "KeepWorld" "KeepWorld" "KeepWorld")
  (`PrimitiveComponent.SetSimulatePhysics` _staticmesh true)
  (`PrimitiveComponent.AddImpulse` _staticmesh Velocity "None" false))

(event `PlaceObject`
  (params (`Socket Transform` :type "Transform Structure") (Socket :type "/Game/Blueprint/Functionality/BP_ItemSocket Object Reference"))
  (`self.K2_DetachFromActor` "KeepWorld" "KeepWorld" "KeepWorld")
  (`self.K2_SetActorTransform` `Socket Transform`))

(fn `UserConstructionScript`)