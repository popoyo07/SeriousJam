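; BP_MoveableWall is a wall actor whose Cube slides along its relative Y axis when something enters the PlayerNear volume.
; Overlap begin plays a whoosh sound and runs the MoveWall timeline, lerping Y from zero to NewLocation; overlap end reverses it.
; No check filters the overlapping actor, and Pushing is cleared just before it is tested, so the guard never blocks.
; BeginPlay creates the audio component and stores a StartingPos that is never read here.
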(event `self.ReceiveBeginPlay`
  (set `self.StartingPos` (`self.GetTransform`))
  (bind _returnvalue (`AddComponent|NODE_AddAudioComponent-0`))
  (set `self.WhooshSFX` _returnvalue))

(event `self.PlayerNear.OnComponentBeginOverlap`
  (params (OverlappedComponent :type "PrimitiveComponent Object Reference") (OtherActor :type "Actor Object Reference") (OtherComp :type "PrimitiveComponent Object Reference") (OtherBodyIndex :type Integer) (bFromSweep :type Boolean) (SweepResult :type "HitResult Structure (by ref)"))
  (set `self.Pushing` false)
  (`AudioComponent.Play` (`self.WhooshSFX`) 0.0)
  (if (not (`self.Pushing`))
    (bind (_direction _movewall_track) (`Timeline|MoveWall` :!label _label)
      (:`Update`
        (`SceneComponent.K2_SetRelativeLocation` (`self.Cube`) (`KismetMathLibrary.MakeVector` 0.0 (`KismetMathLibrary.Lerp` 0.0 (`self.NewLocation`) _movewall_track)) false false))
      (:`Finished`
        (set `self.Pushing` true)))))

(event `self.PlayerNear.OnComponentEndOverlap`
  (params (OverlappedComponent :type "PrimitiveComponent Object Reference") (OtherActor :type "Actor Object Reference") (OtherComp :type "PrimitiveComponent Object Reference") (OtherBodyIndex :type Integer))
  (goto _label :!via `Reverse`))

(fn `UserConstructionScript`)