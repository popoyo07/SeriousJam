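; Spike trap that rises when the player enters its trigger and damages them on contact.
; A TriggerSpikes overlap plays a sound and runs a timeline that sweeps the actor from its start to the DestinedLocation component's position.
; A separate Box overlap calls the first-person character's TakeDamage once, guarded by a flag that is never cleared.
; The player's respawn event teleports the spikes back, stops the sound and re-arms the trigger.
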(event `self.ReceiveBeginPlay`
  (bind _asbp_first_person_character (cast `/Game/FirstPerson/Blueprints/BP_FirstPersonCharacter` (`GameplayStatics.GetPlayerPawn` 0)))
  (bind _output_get (set `self.Player` _asbp_first_person_character))
  (add `/Game/FirstPerson/Blueprints/BP_FirstPersonCharacter.Respawn` _output_get (delegate `ResetSpikes`))
  (set `self.StartingLocation` (`self.K2_GetActorLocation`))
  (set `self.SpikesDesiredLocation` (`SceneComponent.K2_GetComponentLocation` (`self.DestinedLocation`)))
  (bind _returnvalue (`AddComponent|NODE_AddAudioComponent-2`))
  (bind _output_get_2 (set `self.SpikeSfX` _returnvalue))
  (`AudioComponent.Stop` _output_get_2))

(event `ResetSpikes`
  (params (SaveGame :type "/Game/Blueprint/Save/BP_Save Object Reference"))
  (`self.K2_SetActorLocation` (`self.StartingLocation`) false true)
  (set `self.Triggering` false)
  (`AudioComponent.Stop` (`self.SpikeSfX`)))

(event `self.TriggerSpikes.OnComponentBeginOverlap`
  (params (OverlappedComponent :type "PrimitiveComponent Object Reference") (OtherActor :type "Actor Object Reference") (OtherComp :type "PrimitiveComponent Object Reference") (OtherBodyIndex :type Integer) (bFromSweep :type Boolean) (SweepResult :type "HitResult Structure (by ref)"))
  (if (== OtherActor (`self.Player`))
    (if (not (`self.Triggering`))
      (`KismetSystemLibrary.PrintString` "Hello")
      ; Play SFX
      (`AudioComponent.Play` (`self.SpikeSfX`) 0.0)
      (set `self.Triggering` true)
      (bind (_direction _newtrack_0) (`Timeline|SpikeGoUp` :!via `PlayFromStart`)
        (:`Update`
          (`self.K2_SetActorLocation` (`KismetMathLibrary.VLerp` (`self.StartingLocation`) (`self.SpikesDesiredLocation`) _newtrack_0) true))))))

(event `self.Box.OnComponentBeginOverlap`
  (params (OverlappedComponent :type "PrimitiveComponent Object Reference") (OtherActor :type "Actor Object Reference") (OtherComp :type "PrimitiveComponent Object Reference") (OtherBodyIndex :type Integer) (bFromSweep :type Boolean) (SweepResult :type "HitResult Structure (by ref)"))
  (if (== OtherActor (`self.Player`))
    (if (not (`self.KilledPlayer`))
      (set `self.KilledPlayer` true)
      (`/Game/FirstPerson/Blueprints/BP_FirstPersonCharacter.TakeDamage` (`self.Player`) "Ouch"))))

(fn `UserConstructionScript`)