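; A flip door that a boulder triggers, followed by a linked chandelier's vertical move.
; The first BP_Boulder to overlap the Box opens it after a delay, with a timeline lerping the mesh's pitch from its starting rotation by YRotation.
; After another delay, a second timeline moves the chandelier, if valid, to the Box's height while keeping its X and Y.
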(event `self.Box.OnComponentBeginOverlap`
  (params (OverlappedComponent :type "PrimitiveComponent Object Reference") (OtherActor :type "Actor Object Reference") (OtherComp :type "PrimitiveComponent Object Reference") (OtherBodyIndex :type Integer) (bFromSweep :type Boolean) (SweepResult :type "HitResult Structure (by ref)"))
  (if (`GameplayStatics.ObjectIsA` OtherActor "/Game/Blueprint/Functionality/Boulder/BP_Boulder.BP_Boulder_C")
    (`/Engine/EditorBlueprintResources/StandardMacros.DoOnce` false
      (:`Completed`
        (`KismetSystemLibrary.Delay` (`self.DelayDuration`))
        (`self.OpenDoor`)))))

(event `OpenDoor`
  (set `self.StartRotation` (`SceneComponent.K2_GetComponentRotation` (`self.StaticMesh`)))
  (bind (_direction _alpha) (`Timeline|FlipTimeline` :!via `PlayFromStart`)
    (:`Update`
      (`SceneComponent.K2_SetWorldRotation` (`self.StaticMesh`) (`self.LerpRotation` _alpha) false false))
    (:`Finished`
      (`self.MoveChand`))))

(event `MoveChand`
  (`KismetSystemLibrary.Delay` (`self.DelayBeforeChand`))
  (bind _chandelier (`self.Chandelier`)
    (:`then`
      (set `self.ChandStart` (`self.K2_GetActorLocation` _chandelier))
      (bind (_direction _alpha) (`Timeline|ChandTimeline` :!via `PlayFromStart`)
        (:`Update`
          (`self.K2_SetActorLocation` (`self.Chandelier`) (`self.LerpChandLocation` _alpha) false false))))
    (:`else`)))

(fn `UserConstructionScript`)