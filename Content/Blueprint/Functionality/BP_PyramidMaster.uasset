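; Pyramid boss actor whose eye tracks the player and which triggers the win screen once it registers two spins.
; Player entry into the FOV volume enables Tick, which aims the eye and checks the spin count; any overlap end disables it.
; RotationCounter overlaps add spins, gated by a hit cooldown timer, while a decay timer clamps the count back to zero.
; On winning, Tick shows the widget after a delay, stops player movement and enables the cursor.
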(event `self.ReceiveBeginPlay`
  (`self.SetActorTickEnabled` false)
  (set `self.TimeBeforeSpinWheresOff` (`self.StartingTimeBetweenHits`))
  (bind _returnvalue (`|CreateWidget` "/Game/Blueprint/UI/WBP_WinScreen.WBP_WinScreen_C"))
  (set `self.WinWidget` _returnvalue)
  (bind _asbp_first_person_character (cast `/Game/FirstPerson/Blueprints/BP_FirstPersonCharacter` (`GameplayStatics.GetPlayerPawn` 0)))
  (set `self.CharRef` _asbp_first_person_character))

(event `self.ReceiveTick`
  (params (DeltaSeconds :type "Float (single-precision)"))
  (bind _returnvalue (`GameplayStatics.GetPlayerController` 0))
  (`SceneComponent.K2_SetWorldRotation` (`self.DungeonMasterEye`) (`KismetMathLibrary.FindLookAtRotation` (`SceneComponent.K2_GetComponentLocation` (`self.DungeonMasterEye`)) (`self.K2_GetActorLocation` (`GameplayStatics.GetPlayerPawn` 0))) false false)
  (if (== (`self.SpinCount`) 2)
    (`KismetSystemLibrary.Delay` 0.5)
    (`UserWidget.AddToViewport` (`self.WinWidget`) 0)
    (`CharacterMovementComponent.SetMovementMode` (`Character.CharacterMovement` (`self.CharRef`)) "MOVE_None" 0)
    (set `PlayerController.bShowMouseCursor` true _returnvalue)
    (`WidgetBlueprintLibrary.SetInputMode_GameAndUIEx` _returnvalue null "DoNotLock" false)
    (`self.SetActorTickEnabled` false)
    (else
      (`KismetSystemLibrary.PrintString` (`KismetStringLibrary.Conv_IntToString` (`self.SpinCount`))))))

(event `self.FOV.OnComponentEndOverlap`
  (params (OverlappedComponent :type "PrimitiveComponent Object Reference") (OtherActor :type "Actor Object Reference") (OtherComp :type "PrimitiveComponent Object Reference") (OtherBodyIndex :type Integer))
  ; Reset Master
  (`self.SetActorTickEnabled` false))

(event `self.FOV.OnComponentBeginOverlap`
  (params (OverlappedComponent :type "PrimitiveComponent Object Reference") (OtherActor :type "Actor Object Reference") (OtherComp :type "PrimitiveComponent Object Reference") (OtherBodyIndex :type Integer) (bFromSweep :type Boolean) (SweepResult :type "HitResult Structure (by ref)"))
  ; Start Master
  (if (== OtherActor (`GameplayStatics.GetPlayerPawn` 0))
    (`self.SetActorTickEnabled` true)))

(event `self.RotationCounter.OnComponentBeginOverlap`
  (params (OverlappedComponent :type "PrimitiveComponent Object Reference") (OtherActor :type "Actor Object Reference") (OtherComp :type "PrimitiveComponent Object Reference") (OtherBodyIndex :type Integer) (bFromSweep :type Boolean) (SweepResult :type "HitResult Structure (by ref)"))
  ; Add to spin count
  (`KismetSystemLibrary.K2_SetTimerDelegate` (delegate `CanHitTime`) (`self.TimeBetweenHits`))
  (if (`self.CanHit`)
    (set `self.SpinCount` (+ (`self.SpinCount`) 1))
    (`KismetSystemLibrary.K2_ClearAndInvalidateTimerHandle` (`self.TimeBetweenSpins`))
    (set `self.CanHit` false)
    (else
      (`KismetSystemLibrary.PrintString` "ToSoon"))))

(event `self.RotationCounter.OnComponentEndOverlap`
  (params (OverlappedComponent :type "PrimitiveComponent Object Reference") (OtherActor :type "Actor Object Reference") (OtherComp :type "PrimitiveComponent Object Reference") (OtherBodyIndex :type Integer))
  ; Remove from spin count
  (bind _returnvalue (`KismetSystemLibrary.K2_SetTimerDelegate` (delegate `Minus1`) (`self.TimeBeforeSpinWheresOff`)))
  (set `self.TimeBetweenSpins` _returnvalue))

(event `Minus1`
  ; Remove from spin count
  (set `self.SpinCount` (`KismetMathLibrary.Clamp` (- (`self.SpinCount`) 1)))
  (set `self.CanHit` true))

(event `CanHitTime`
  ; Add to spin count
  (set `self.CanHit` true))

(fn `UserConstructionScript`)