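; BP_Rotation is a component that spins its owning actor around the local roll axis.
; The Rotating event sets angular velocity from the input's roll value scaled by a rotation speed.
; While velocity is nonzero, Tick applies it times a damping factor, without delta time or decay.
; It also fires the RotatingValid dispatcher each tick, true only when that signed step exceeds a fixed threshold.
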(event `self.ReceiveBeginPlay`)

(event `self.ReceiveTick`
  (params (DeltaSeconds :type "Float (single-precision)"))
  (bind _returnvalue (* (`self.AngularVelocity`) (`self.Damping`)))
  (if (!= (`self.AngularVelocity`) 0.0)
    (`Actor.K2_AddActorLocalRotation` (`self.GetOwner`) (`KismetMathLibrary.MakeRotator` _returnvalue) false false)
    (if (> _returnvalue 1.5)
      (`self.rotatingValid` true)
      (else
        (`self.rotatingValid` false)))))

(event `Rotating`
  (params (TargetVector :type "Rotator Structure"))
  (set `self.AngularVelocity` (* TargetVector_Roll (`self.RotationSpeed`))))