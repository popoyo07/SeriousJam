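; BP_SpawnBoulder is a trigger-driven boulder trap that spawns a BP_Boulder at its SpawnPoint on BeginPlay, hidden and without physics.
; When the player enters its Box, the boulder becomes visible, active and physics-simulated.
; A Reset bound through the character's AssignRespawn disables the boulder and returns it to SpawnPoint.
; The timed respawn and the setting of the BoulderActiviate guard are disconnected, so neither runs.
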(event `BoulderEnable`
  (params (isAble :type Boolean))
  (bind _boulder (`self.Boulder`))
  (bind _boulder_2 (`/Game/Blueprint/Functionality/Boulder/BP_Boulder.Boulder` _boulder))
  (`SceneComponent.SetVisibility` _boulder_2 isAble false)
  (set `/Game/Blueprint/Functionality/Boulder/BP_Boulder.isActiving` isAble _boulder)
  (`PrimitiveComponent.SetSimulatePhysics` _boulder_2 isAble))

(event `self.ReceiveBeginPlay`
  (`self.SpawnBoulder`)
  (`self.BoulderEnable` false)
  (bind _asbp_first_person_character (cast `/Game/FirstPerson/Blueprints/BP_FirstPersonCharacter` (`GameplayStatics.GetPlayerCharacter` 0)))
  (set `self.As BP First Person Character` _asbp_first_person_character)
  (add `/Game/FirstPerson/Blueprints/BP_FirstPersonCharacter.Respawn` (`self.As BP First Person Character`) (delegate `Reset`)))

(event `Reset`
  (params (SaveGame :type "/Game/Blueprint/Save/BP_Save Object Reference"))
  (`self.BoulderEnable` false)
  (`SceneComponent.K2_SetWorldTransform` (`/Game/Blueprint/Functionality/Boulder/BP_Boulder.Boulder` (`self.Boulder`)) (`SceneComponent.K2_GetComponentToWorld` (`self.SpawnPoint`)) false false)
  (set `self.BoulderActiviate` false))

(event `SpawnBoulder`
  (bind _returnvalue (`|SpawnActorFromClass` "/Game/Blueprint/Functionality/Boulder/BP_Boulder.BP_Boulder_C" (`SceneComponent.K2_GetComponentToWorld` (`self.SpawnPoint`)) "Undefined" "MultiplyWithRoot" null null))
  (set `self.Boulder` _returnvalue))

(event `self.Box.OnComponentBeginOverlap`
  (params (OverlappedComponent :type "PrimitiveComponent Object Reference") (OtherActor :type "Actor Object Reference") (OtherComp :type "PrimitiveComponent Object Reference") (OtherBodyIndex :type Integer) (bFromSweep :type Boolean) (SweepResult :type "HitResult Structure (by ref)"))
  (if (== OtherActor (`self.As BP First Person Character`))
    (if (not (`self.BoulderActiviate`))
      (`self.BoulderEnable` true))))

(fn `UserConstructionScript`)