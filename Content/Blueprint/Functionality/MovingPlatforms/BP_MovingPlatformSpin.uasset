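; Moving platform that spins faster and shifts vertically while something overlaps its trigger Box.
; Box overlap raises the RotatingMovement rate, plays a spin sound and runs a Timeline that lerps the Cube's relative Z toward Distance.
; End overlap lowers the spin rate and reverses the Timeline to return the Cube.
; The SpinSFX audio component is created at BeginPlay, and overlaps are not filtered by actor.
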(event `self.ReceiveBeginPlay`
  (bind _returnvalue (`AddComponent|NODE_AddAudioComponent-0`))
  (set `self.SpinSFX` _returnvalue))

(event `self.Box.OnComponentBeginOverlap`
  (params (OverlappedComponent :type "PrimitiveComponent Object Reference") (OtherActor :type "Actor Object Reference") (OtherComp :type "PrimitiveComponent Object Reference") (OtherBodyIndex :type Integer) (bFromSweep :type Boolean) (SweepResult :type "HitResult Structure (by ref)"))
  (`AudioComponent.Play` (`self.SpinSFX`) 0.0)
  (set `RotatingMovementComponent.RotationRate` (struct :`Yaw` 400.0) (`self.RotatingMovement`))
  (bind (_direction _movewall_track) (`Timeline|Timeline` :!label _label)
    (:`Update`
      (`SceneComponent.K2_SetRelativeLocation` (`self.Cube`) (`KismetMathLibrary.MakeVector` 0.0 0.0 (`KismetMathLibrary.Lerp` 0.0 (`self.Distance`) _movewall_track)) false false))))

(event `self.Box.OnComponentEndOverlap`
  (params (OverlappedComponent :type "PrimitiveComponent Object Reference") (OtherActor :type "Actor Object Reference") (OtherComp :type "PrimitiveComponent Object Reference") (OtherBodyIndex :type Integer))
  (set `RotatingMovementComponent.RotationRate` (struct :`Yaw` 200.0) (`self.RotatingMovement`))
  (goto _label :!via `Reverse`))

(fn `UserConstructionScript`)