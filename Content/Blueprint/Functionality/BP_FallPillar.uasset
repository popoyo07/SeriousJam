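; BP_FallPillar is a pillar trap that tips over and squashes the player when its Box trigger is overlapped while IsTrap is set.
; After a short delay it plays a sound, snaps by a configurable local rotation, damages the cached first-person character, then rotates back after a pause.
; The overlap does not check which actor entered, and damage always goes to that character, with no second hit test.
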(event `self.ReceiveBeginPlay`
  (bind _asbp_first_person_character (cast `/Game/FirstPerson/Blueprints/BP_FirstPersonCharacter` (`GameplayStatics.GetPlayerPawn` 0)))
  (set `self.CharRef` _asbp_first_person_character)
  (bind _returnvalue (`AddComponent|NODE_AddAudioComponent-1`))
  (set `self.SFX` _returnvalue))

(event `self.Box.OnComponentBeginOverlap`
  (params (OverlappedComponent :type "PrimitiveComponent Object Reference") (OtherActor :type "Actor Object Reference") (OtherComp :type "PrimitiveComponent Object Reference") (OtherBodyIndex :type Integer) (bFromSweep :type Boolean) (SweepResult :type "HitResult Structure (by ref)"))
  (if (`self.isTrap`)
    (`KismetSystemLibrary.Delay` 0.2)
    (`AudioComponent.Play` (`self.SFX`) 0.0)
    (`self.K2_AddActorLocalRotation` (`KismetMathLibrary.MakeRotator` (`self.BeginRotation X (Roll)`) (`self.BeginRotation Y (Pitch)`) (`self.BeginRotation Z (Yaw)`)))
    (`KismetSystemLibrary.Delay` 0.2)
    (`/Game/FirstPerson/Blueprints/BP_FirstPersonCharacter.TakeDamage` (`self.CharRef`) "Squashed by Pillar")
    (`KismetSystemLibrary.Delay` 2.0)
    (`self.K2_AddActorLocalRotation` (`KismetMathLibrary.MakeRotator` (* (`self.BeginRotation X (Roll)`) -1.0) (* (`self.BeginRotation Y (Pitch)`) -1.0) (* (`self.BeginRotation Z (Yaw)`) -1.0)))))

(fn `UserConstructionScript`)