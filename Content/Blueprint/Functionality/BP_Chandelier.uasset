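; Chandelier actor the player can grab, which spins with the player attached and then drops after a timed delay.
; Proximity volumes toggle tick and the grab prompt widget.
; While attached, tick-driven Spin eases the camera toward the character's rotation and drives rotating movement.
; After the delay it enables physics, detaches the player into falling, plays fall audio, stops ticking, and later disables physics.
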(event `self.ReceiveBeginPlay`
  (bind _asbp_first_person_character (cast `/Game/FirstPerson/Blueprints/BP_FirstPersonCharacter` (`GameplayStatics.GetPlayerPawn` 0)))
  (set `self.CharRef` _asbp_first_person_character)
  (bind _returnvalue (`AddComponent|NODE_AddAudioComponent-1`))
  (set `self.ChandSpinSFX` _returnvalue)
  (bind _returnvalue_2 (`AddComponent|NODE_AddAudioComponent-0`))
  (set `self.FallingSFX` _returnvalue_2))

(event `self.ReceiveTick`
  (params (DeltaSeconds :type "Float (single-precision)"))
  (`self.Spin`))

(event `self.PlayerNear.OnComponentEndOverlap`
  (params (OverlappedComponent :type "PrimitiveComponent Object Reference") (OtherActor :type "Actor Object Reference") (OtherComp :type "PrimitiveComponent Object Reference") (OtherBodyIndex :type Integer))
  (if (== OtherActor (`GameplayStatics.GetPlayerPawn` 0))
    (`self.SetActorTickEnabled` false)))

(event `self.PlayerNear.OnComponentBeginOverlap`
  (params (OverlappedComponent :type "PrimitiveComponent Object Reference") (OtherActor :type "Actor Object Reference") (OtherComp :type "PrimitiveComponent Object Reference") (OtherBodyIndex :type Integer) (bFromSweep :type Boolean) (SweepResult :type "HitResult Structure (by ref)"))
  (if (== OtherActor (`GameplayStatics.GetPlayerPawn` 0))
    (`self.SetActorTickEnabled` true)))

(event `Spin`
  (bind _charref (`self.CharRef`))
  (bind _charref_2 (`self.CharRef`))
  (if (`/Game/FirstPerson/Blueprints/BP_FirstPersonCharacter.IsAttachedToChandelier?` (`self.CharRef`))
    (`SceneComponent.SetHiddenInGame` (`self.Widget`) true false)
    (`Controller.SetControlRotation` (`GameplayStatics.GetPlayerController` 0) (`KismetMathLibrary.RInterpTo` (`SceneComponent.K2_GetComponentRotation` (`JamCharacter.FirstPersonCameraComponent` _charref)) (`self.K2_GetActorRotation` _charref) (`GameplayStatics.GetWorldDeltaSeconds`) 2.0))
    (set `RotatingMovementComponent.RotationRate` (struct :`Yaw` 600.0) (`self.RotatingMovement`))
    (`KismetSystemLibrary.Delay` (`self.TimeUntilDrop`))
    (`PrimitiveComponent.SetSimulatePhysics` (`self.Sphere`) true)
    (`CharacterMovementComponent.SetMovementMode` (`Character.CharacterMovement` _charref_2) "MOVE_Falling" 0)
    (`AudioComponent.Play` (`self.FallingSFX`) 0.0)
    (`/Game/FirstPerson/Blueprints/BP_FirstPersonCharacter.DetachFromChand` _charref_2)
    (`self.SetActorTickEnabled` false)
    (`KismetSystemLibrary.Delay` (`self.TimeUntilHitFloorAfterDrop`))
    (`PrimitiveComponent.SetSimulatePhysics` (`self.Sphere`) false)
    (set `/Game/FirstPerson/Blueprints/BP_FirstPersonCharacter.IsAttachedToChandelier?` false (`self.CharRef`))))

(event `self.GToGrab.OnComponentBeginOverlap`
  (params (OverlappedComponent :type "PrimitiveComponent Object Reference") (OtherActor :type "Actor Object Reference") (OtherComp :type "PrimitiveComponent Object Reference") (OtherBodyIndex :type Integer) (bFromSweep :type Boolean) (SweepResult :type "HitResult Structure (by ref)"))
  (if (== OtherActor (`GameplayStatics.GetPlayerPawn` 0))
    (`SceneComponent.SetHiddenInGame` (`self.Widget`) false false)
    (`KismetSystemLibrary.PrintString` "Hello")))

(event `PlaySpinSFX`
  (`AudioComponent.Play` (`self.ChandSpinSFX`) 0.0))

(event `self.GToGrab.OnComponentEndOverlap`
  (params (OverlappedComponent :type "PrimitiveComponent Object Reference") (OtherActor :type "Actor Object Reference") (OtherComp :type "PrimitiveComponent Object Reference") (OtherBodyIndex :type Integer))
  (if (== OtherActor (`GameplayStatics.GetPlayerPawn` 0))
    (`SceneComponent.SetHiddenInGame` (`self.Widget`) true false)))

(fn `UserConstructionScript`)