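; BP_Checkpoint is a trigger actor that sets the player's checkpoint and saves the game when the player overlaps it.
; On BeginPlay it caches references to the first-person character and BP_GameInstance.
; When the player pawn enters SaveCollider and the game instance is not loading, it registers itself as the current checkpoint, calls SaveGame and plays a 2D sound.
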(event `self.ReceiveBeginPlay`
  (bind _asbp_first_person_character (cast `/Game/FirstPerson/Blueprints/BP_FirstPersonCharacter` (`GameplayStatics.GetPlayerPawn` 0)))
  (set `self.CharRef` _asbp_first_person_character)
  (bind _asbp_game_instance (cast `/Game/FirstPerson/Blueprints/BP_GameInstance` (`GameplayStatics.GetGameInstance`)))
  (set `self.GameIns` _asbp_game_instance))

(event `self.SaveCollider.OnComponentBeginOverlap`
  (params (OverlappedComponent :type "PrimitiveComponent Object Reference") (OtherActor :type "Actor Object Reference") (OtherComp :type "PrimitiveComponent Object Reference") (OtherBodyIndex :type Integer) (bFromSweep :type Boolean) (SweepResult :type "HitResult Structure (by ref)"))
  (bind _gameins (`self.GameIns`))
  ; Set spawnpoint
  (if (== OtherActor (`GameplayStatics.GetPlayerPawn` 0))
    (if (not (`/Game/FirstPerson/Blueprints/BP_GameInstance.IsLoading` (`self.GameIns`)))
      (set `/Game/FirstPerson/Blueprints/BP_GameInstance.Checkpoint` self _gameins)
      (`/Game/FirstPerson/Blueprints/BP_GameInstance.SaveGame` _gameins)
      (`GameplayStatics.PlaySound2D` "/Game/Weapons/GrenadeLauncher/Audio/FirstPersonTemplateWeaponFire02.FirstPersonTemplateWeaponFire02" 1.0 1.0 0.0 null null))))

(fn `UserConstructionScript`)