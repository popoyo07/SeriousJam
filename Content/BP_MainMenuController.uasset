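; Main menu controller that lets the player click and spin interactable objects.
; IA_ClickToSpin traces under the cursor for a "CanInteract"-tagged actor, stores it, plays an audio component added at BeginPlay and sets a spin flag until release.
; While that flag is set, IA_SpinObject passes input X/Y as roll and pitch to the object's BP_Rotation component.
; Debug strings print the spin state and input.
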(event `self.ReceiveBeginPlay`
  (bind _returnvalue (`AddComponent|NODE_AddAudioComponent-0`))
  (set `self.SFX` _returnvalue))

(event `EnhancedInput|/Game/Input/Actions/IA_UI/IA_SpinObject`
  (params (ActionValue :type "Vector2D Structure") (ElapsedSeconds :type "Float (double-precision)") (TriggeredSeconds :type "Float (double-precision)") (InputAction :type "InputAction Object Reference" :default "/Game/Input/Actions/IA_UI/IA_SpinObject.IA_SpinObject"))
  (bind (_x _y) (`KismetMathLibrary.BreakVector2D` ActionValue))
  (:`Ongoing`
    (if (`self.isSpawing`)
      (`/Game/Blueprint/Functionality/BP_Rotation.Rotating` (`self.GetComponentByClass` (`self.CurrentObject`) "/Game/Blueprint/Functionality/BP_Rotation.BP_Rotation_C") (`KismetMathLibrary.MakeRotator` _x _y))
      (`KismetSystemLibrary.PrintString` (`KismetStringLibrary.Concat_StrStr` (`KismetStringLibrary.Conv_DoubleToString` _x))))))

(event `EnhancedInput|/Game/Input/Actions/IA_UI/IA_ClickToSpin`
  (params (ActionValue :type Boolean) (ElapsedSeconds :type "Float (double-precision)") (TriggeredSeconds :type "Float (double-precision)") (InputAction :type "InputAction Object Reference" :default "/Game/Input/Actions/IA_UI/IA_ClickToSpin.IA_ClickToSpin"))
  (bind _hitresult (`self.GetHitResultUnderCursorByChannel` (`GameplayStatics.GetPlayerController` 0) "TraceTypeQuery1" true))
  (:`Started`
    (if (`self.ActorHasTag` (`.HitActor` (`GameplayStatics.BreakHitResult` _hitresult)) "CanInteract")
      (set `self.CurrentObject` (`.HitActor` (`GameplayStatics.BreakHitResult` _hitresult)))
      (set `self.isSpawing` true)
      (`AudioComponent.Play` (`self.SFX`) 0.0)
      (`KismetSystemLibrary.PrintString` "ReadyToSpin")
      (else
        (`KismetSystemLibrary.PrintString` "NoSpin" :!label _label))))
  (:`Completed`
    (set `self.isSpawing` false)
    (goto _label)))

(fn `UserConstructionScript`)